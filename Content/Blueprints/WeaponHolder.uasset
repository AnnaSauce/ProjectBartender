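; WeaponHolder is a scene component that spawns, holds and switches its owner's weapon.
; It spawns the selected class from UnlockedWeapons and attaches it to itself, destroying and respawning as selection wraps around the list.
; Trigger input converts a performance grade into a ricochet count for the top grades, then fires and plays a gunshot or cork sound depending on success.
; Reload input is forwarded to the weapon.
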(event `self.ReceiveBeginPlay`
  (`self.Initialise Weapon` (`self.Selected Weapon`)))

(event `TriggerDown`
  (params (Reticle :type "Vector Structure") (Direction :type "Vector Structure") (Grade :type "/Game/Blueprints/Score/Grade Enum" :default "NewEnumerator0"))
  (bind _weapon (`self.Weapon`))
  (bind _returnvalue (`Actor.K2_GetActorLocation` _weapon))
  ;[1 1 1] If there is a weapon, shoot it
  (`/Engine/EditorBlueprintResources/StandardMacros.IsValid` _weapon
    (:`Is Valid`
      (switch `/Game/Blueprints/Score/Grade` Grade
        (:`NewEnumerator0`
          (set `self.Times to Ricochet` 3))
        (:`NewEnumerator1`
          (set `self.Times to Ricochet` 1))
        (:`NewEnumerator2`
          _)
        (:`NewEnumerator3`
          _)
        (:`NewEnumerator4`
          _))
      (bind _returnvalue_2 (`Weapon.TryFiring` _weapon Reticle Direction (`self.Times to Ricochet`)))
      (if _returnvalue_2
        (`GameplayStatics.PlaySoundAtLocation` "/Game/Audio/SFX/GunShot.GunShot" _returnvalue (struct) 1.0 1.0 0.0 null null null null)
        (else
          (`GameplayStatics.PlaySoundAtLocation` "/Game/Audio/SFX/GunCork.GunCork" _returnvalue (struct) 1.0 1.0 0.0 null null null null))))))

(event `ReloadPressed`
  ;[0 0.5176 1] If the weapons current ammo count is less than its max capacity...
  (`Weapon.Reload` (`self.Weapon`)))

(fn `Initialise Weapon`
  (params (`Selected Weapon Index` :type Integer))
  (bind _returnvalue (`|SpawnActorFromClass` (`|GetArrayItem` (`self.UnlockedWeapons`) `Selected Weapon Index`) (`self.GetRelativeTransform`) "AlwaysSpawn" "MultiplyWithRoot" (`self.GetOwner`) null))
  (bind _output_get (set `self.Weapon` _returnvalue))
  (`Actor.K2_AttachToComponent` _output_get self "None" "KeepRelative" "KeepRelative" "KeepRelative" true))

(fn `Switch Weapon`
  (params (Direction :type "Float (double-precision)"))
  ;[1 1 1] Destroys weapon and uses an int to move to the next slot and spawns the new weapon.
  (`Actor.K2_DestroyActor` (`self.Weapon`))
  (if (> Direction 0.0)
    (if (== (`self.Selected Weapon`) (`KismetArrayLibrary.Array_LastIndex` (`self.UnlockedWeapons`)))
      (bind _output_get (set `self.Selected Weapon` 0))
      (else
        (`/Engine/EditorBlueprintResources/StandardMacros.IncrementInt` _output_get
          (:`  `
            _))))
    (elif (== (`self.Selected Weapon`) 0)
      (bind _output_get_2 (set `self.Selected Weapon` (`KismetArrayLibrary.Array_LastIndex` (`self.UnlockedWeapons`))))
      (else
        (`/Engine/EditorBlueprintResources/StandardMacros.DecrementInt` _output_get_2
          (:`  `
            _)))))
  (`self.Initialise Weapon` (`self.Selected Weapon`)))