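; BP_Sentry is an enemy that fires bursts of BP_Bullets when it sees the player and is destroyed when damage depletes its health.
; PawnSensing sightings drive delayed shots from an Arrow component, counting down the burst before a reload delay refills it.
; Each sighting also sets rotation with a look-at, but both endpoints are the seen player's location, so it does not aim from the sentry.
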(event `self.ReceiveBeginPlay`
  (set `self.BurstAmmount` (`self.BurstMax`)))

(event `self.ReceiveAnyDamage`
  (params (Damage :type "Float (single-precision)") (DamageType :type "DamageType Object Reference") (InstigatedBy :type "Controller Object Reference") (DamageCauser :type "Actor Object Reference"))
  (bind _output_get (set `self.Health` (- (`self.Health`) Damage)))
  (if (<= _output_get 0.0)
    (`self.Death`)))

(event `Death`
  (bind _output_get (set `self.Health` (`self.Health`)))
  (if (<= _output_get 0.0)
    (`self.K2_DestroyActor`)))

(event `self.PawnSensing.OnSeePawn`
  (params (Pawn :type "Pawn Object Reference"))
  (bind _asbp_player_character (cast `/Game/Blueprints/BP_PlayerCharacter` Pawn))
  (`self.K2_SetActorRotation` (`KismetMathLibrary.FindLookAtRotation` (`self.K2_GetActorLocation` _asbp_player_character) (`self.K2_GetActorLocation` Pawn)))
  (if (>= (`self.BurstAmmount`) 0)
    (`KismetSystemLibrary.Delay` (`self.FireRate`))
    (`|SpawnActorFromClass` "/Game/Blueprints/Enemies/BP_Bullets.BP_Bullets_C" (`SceneComponent.K2_GetComponentToWorld` (`self.Arrow`)) "AdjustIfPossibleButAlwaysSpawn" "MultiplyWithRoot" null null)
    (`/Engine/EditorBlueprintResources/StandardMacros.DecrementInt` (`self.BurstAmmount`))
    (else
      (`KismetSystemLibrary.Delay` (`self.ReloadTime`))
      (set `self.BurstAmmount` (`self.BurstMax`)))))

(fn `UserConstructionScript`)