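; BP_DroneController is the AI controller for drone enemies, running the prototype drone behavior tree on BeginPlay.
; Its perception update handler filters for sight stimuli from the first player character.
; It writes that player to the PlayerTarget blackboard key when sensed and clears the key when sight is lost.
; Debug prints mark perception updates and player sight events.
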(event `self.ReceiveBeginPlay`
  (`self.RunBehaviorTree` "/Game/Blueprints/Enemies/AI_Behaviour/Drone/BT_DronePrototype.BT_DronePrototype"))

(event `self.AIPerception.OnTargetPerceptionUpdated`
  (params (Actor :type "Actor Object Reference") (Stimulus :type "AIStimulus Structure"))
  (`KismetSystemLibrary.PrintString` "Hello")
  (bind _returnvalue (`AIPerceptionSystem.GetSenseClassForStimulus` Stimulus))
  (if (== _returnvalue "/Script/AIModule.AISense_Sight")
    (if (== Actor (`GameplayStatics.GetPlayerCharacter` 0))
      (`BlackboardComponent.SetValueAsObject` (`self.Blackboard`) "PlayerTarget" (`KismetMathLibrary.SelectObject` Actor null (`.bSuccessfullySensed` (break `AIStimulus` Stimulus))))
      (`KismetSystemLibrary.PrintString` "seen"))))

(fn `UserConstructionScript`)