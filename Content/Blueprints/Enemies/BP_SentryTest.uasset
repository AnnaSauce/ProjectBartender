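; BP_SentryTest is an enemy sentry that shoots at the player and can be destroyed.
; When PawnSensing sees a BP_PlayerCharacter, it snaps to face the player, waits briefly, then spawns BP_Bullets at its Arrow transform.
; Any damage reduces Health, and Death destroys the actor once Health reaches zero or below.
; BeginPlay switches on TurretStates, but no branch does anything.
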(event `self.ReceiveAnyDamage`
  (params (Damage :type "Float (single-precision)") (DamageType :type "DamageType Object Reference") (InstigatedBy :type "Controller Object Reference") (DamageCauser :type "Actor Object Reference"))
  (bind _output_get (set `self.Health` (- (`self.Health`) Damage)))
  (if (<= _output_get 0.0)
    (`self.Death`)))

(event `Death`
  (bind _output_get (set `self.Health` (`self.Health`)))
  (if (<= _output_get 0.0)
    (`self.K2_DestroyActor`)))

(event `self.PawnSensing.OnSeePawn`
  (params (Pawn :type "Pawn Object Reference"))
  (cast `/Game/Blueprints/BP_PlayerCharacter` Pawn)
  (`self.K2_SetActorRotation` (`KismetMathLibrary.FindLookAtRotation` (`self.K2_GetActorLocation`) (`self.K2_GetActorLocation` Pawn)))
  (`KismetSystemLibrary.Delay` 0.2)
  (`|SpawnActorFromClass` "/Game/Blueprints/Enemies/BP_Bullets.BP_Bullets_C" (`SceneComponent.K2_GetComponentToWorld` (`self.Arrow`)) "AdjustIfPossibleButAlwaysSpawn" "MultiplyWithRoot" null null))

(event `self.ReceiveBeginPlay`
  (switch `/Game/Blueprints/Enemies/AI_Behaviour/Sentry/Turret_States` (`self.TurretStates`)))

(fn `UserConstructionScript`)