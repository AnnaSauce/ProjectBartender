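; Drone enemy prototype with a timeline-driven rotor spin, health and point rewards through GM_Gameplay.
; AnyDamage reduces health; death stops the rotor, enables physics on its parts, disables other collision, awards points and expires after a delay.
; ManageCriticalHit awards hit points while alive, more for criticals.
; PawnSensing sets a look-at rotation on seeing the player, but both look-at endpoints are the player's location.
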(event `self.ReceiveBeginPlay`
  (`self.Rotate`)
  (bind _asgm_gameplay (cast `/Game/Blueprints/GameManagement/GM_Gameplay` (`GameplayStatics.GetGameMode`)))
  (set `self.gameMode` _asgm_gameplay))

(event `Rotate`
  ;[1 0.8195 0.3199] ProperllorSpin
  (bind _output_get (set `self.startRot` (`SceneComponent.K2_GetComponentRotation` (`self.Rotor`))))
  (set `self.endRot` (`KismetMathLibrary.MakeRotator` (.roll _output_get) (.pitch _output_get) (+ (.yaw _output_get) 360.0)))
  (bind (_direction _rottrack) (`Timeline|Rotate_TML` :!via `PlayFromStart` :!label _label)
    (:`Update`
      (`SceneComponent.K2_SetWorldRotation` (`self.Rotor`) (`KismetMathLibrary.RLerp` (`self.startRot`) (`self.endRot`) _rottrack) false false))))

(event `StopRotate`
  ;[1 0.8195 0.3199] ProperllorSpin
  (goto _label :!via `Stop`))

(event `self.ReceiveAnyDamage`
  (params (Damage :type "Float (single-precision)") (DamageType :type "DamageType Object Reference") (InstigatedBy :type "Controller Object Reference") (DamageCauser :type "Actor Object Reference"))
  ;[1 0.1265 0.1265] Damage and Death
  (bind _output_get (set `self.health` (- (`self.health`) Damage)))
  (if (<= _output_get 0.0)
    (`self.Death`)))

(event `Death`
  ;[1 0.1265 0.1265] Damage and Death
  (`self.SetLifeSpan` 3.0)
  (`PrimitiveComponent.SetSimulatePhysics` (`self.Sphere`) true)
  (`PrimitiveComponent.SetSimulatePhysics` (`self.Rotor`) true)
  (`PrimitiveComponent.SetSimulatePhysics` (`self.Cylinder1`) true)
  (`self.StopRotate`)
  (`/Game/Blueprints/GameManagement/GM_Gameplay.Send Points To Player` (`self.gameMode`) 15)
  (`PrimitiveComponent.SetCollisionEnabled` (`self.Capsule`) "NoCollision")
  (`PrimitiveComponent.SetCollisionEnabled` (`self.Box`) "NoCollision"))

(event `/Game/Blueprints/BPI_Hitbox.ManageCriticalHit`
  (params (`Critical Hit?` :type Boolean))
  (bind _gamemode (`self.gameMode`))
  (if (> (`self.health`) 0.0)
    (if `Critical Hit?`
      (`/Game/Blueprints/GameManagement/GM_Gameplay.Send Points To Player` _gamemode 10)
      (else
        (`/Game/Blueprints/GameManagement/GM_Gameplay.Send Points To Player` _gamemode 5)))))

(event `self.PawnSensing.OnSeePawn`
  (params (Pawn :type "Pawn Object Reference"))
  (bind _asbp_player_character (cast `/Game/Blueprints/BP_PlayerCharacter` Pawn))
  (`self.K2_SetActorRotation` (`KismetMathLibrary.FindLookAtRotation` (`self.K2_GetActorLocation` _asbp_player_character) (`self.K2_GetActorLocation` Pawn))))

(fn `UserConstructionScript`)