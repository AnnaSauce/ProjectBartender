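; Scene component that holds its owner's active weapon, forwarding fire, stop and reload input to it.
; On BeginPlay it spawns the selected class from UnlockedWeapons and attaches it to itself.
; SwitchWeapon destroys the current weapon, steps the index up or down with wraparound, and spawns the replacement.
; Spawned weapons take the component's owner as Owner, which a comment notes hitscan line traces rely on.
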(event `self.ReceiveBeginPlay`
  (`self.Initialise Weapon` (`self.Selected Weapon`)))

(event `TriggerDown`
  (params (Reticle :type "Vector Structure") (Direction :type "Vector Structure"))
  (bind _weapon (`self.Weapon`))
  ;[1 1 1] If there is a weapon, shoot it
  (`/Engine/EditorBlueprintResources/StandardMacros.IsValid` _weapon
    (:`Is Valid`
      (`Weapon_Base.Fire` _weapon Reticle Direction))))

(event `TriggerUp`
  (bind _weapon (`self.Weapon`))
  ;[1 1 1] If there is a weapon, shoot it
  (`/Engine/EditorBlueprintResources/StandardMacros.IsValid` _weapon
    (:`Is Valid`
      (`Weapon_Base.StopFiring` _weapon))))

(event `ReloadPressed`
  ;[0 0.5176 1] If the weapons current ammo count is less than its max capacity...
  (`Weapon_Base.Reload` (`self.Weapon`)))

(fn `Initialise Weapon`
  (params (`Selected Weapon Index` :type Integer))
  (bind _returnvalue (`|SpawnActorFromClass` (`|GetArrayItem` (`self.UnlockedWeapons`) `Selected Weapon Index`) (`self.GetRelativeTransform`) "AlwaysSpawn" "MultiplyWithRoot" (`self.GetOwner`) null))
  (bind _output_get (set `self.Weapon` _returnvalue))
  (`Actor.K2_AttachToComponent` _output_get self "None" "KeepRelative" "KeepRelative" "KeepRelative" true))

(fn `Switch Weapon`
  (params (Direction :type "Float (double-precision)"))
  ;[1 1 1] Destroys weapon and uses an int to move to the next slot and spawns the new weapon.
  (`Actor.K2_DestroyActor` (`self.Weapon`))
  (if (> Direction 0.0)
    (if (== (`self.Selected Weapon`) (`KismetArrayLibrary.Array_LastIndex` (`self.UnlockedWeapons`)))
      (bind _output_get (set `self.Selected Weapon` 0))
      (else
        (`/Engine/EditorBlueprintResources/StandardMacros.IncrementInt` _output_get
          (:`  `
            _))))
    (elif (== (`self.Selected Weapon`) 0)
      (bind _output_get_2 (set `self.Selected Weapon` (`KismetArrayLibrary.Array_LastIndex` (`self.UnlockedWeapons`))))
      (else
        (`/Engine/EditorBlueprintResources/StandardMacros.DecrementInt` _output_get_2
          (:`  `
            _)))))
  (`self.Initialise Weapon` (`self.Selected Weapon`)))