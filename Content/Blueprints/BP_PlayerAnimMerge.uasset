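; Player character Blueprint with look, move, double jump, sprint toggle, camera-drop slide, audio, weapon input, health and pause menu.
; Hits on "Wallrunable"-tagged actors start wallruns using a movement plane constraint, reduced gravity, camera tilt and a launch.
; Tick ends wallruns when trace, falling, speed or facing checks fail, while jumping launches off the wall.
; Weapon input forwards to WeaponHolder, and damage only lowers and prints Health.
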(event `self.ReceiveTick`
  (params (DeltaSeconds :type "Float (single-precision)"))
  ;[1 0 0.07548] Tick
  (`self.Update Wallrunning`))

(event `EnhancedInput|/Game/Input/Actions/Action_Look`
  (params (ActionValue :type "Vector2D Structure") (ElapsedSeconds :type "Float (double-precision)") (TriggeredSeconds :type "Float (double-precision)") (InputAction :type "InputAction Object Reference" :default "/Game/Input/Actions/Action_Look.Action_Look"))
  ;[1 1 1] Camera Action - JR
  (:`Triggered`
    (`self.AddControllerYawInput` ActionValue_X)
    (`self.AddControllerPitchInput` (* ActionValue_Y -1.0))))

(event `EnhancedInput|/Game/Input/Actions/Action_Move`
  (params (ActionValue :type "Vector2D Structure") (ElapsedSeconds :type "Float (double-precision)") (TriggeredSeconds :type "Float (double-precision)") (InputAction :type "InputAction Object Reference" :default "/Game/Input/Actions/Action_Move.Action_Move"))
  ;[1 1 1] Movement Action - AV
  (:`Triggered`
    (`self.AddMovementInput` (`self.GetActorRightVector`) ActionValue_X)
    (`self.AddMovementInput` (`self.GetActorForwardVector`) ActionValue_Y)
    ;[1 0.09393 0] Walk/Run Cycle Audio
    (`/Engine/EditorBlueprintResources/StandardMacros.DoOnce` false :!label _label
      (:`Completed`
        (`GameplayStatics.PlaySoundAtLocation` "/Game/Audio/SFX/StepSound.StepSound" (`SceneComponent.K2_GetComponentLocation` (`self.Camera`)) (struct) 1.0 1.0 0.0 null null null null)
        (if (`self.is_Sprinting`)
          (`KismetSystemLibrary.Delay` 0.25)
          (goto _label :!via `Reset`)
          (else
            (`KismetSystemLibrary.Delay` 0.5)
            (goto _label :!via `Reset`)))))))

(event `EnhancedInput|/Game/Input/Actions/Action_Jump`
  (params (ActionValue :type Boolean) (ElapsedSeconds :type "Float (double-precision)") (TriggeredSeconds :type "Float (double-precision)") (InputAction :type "InputAction Object Reference" :default "/Game/Input/Actions/Action_Jump.Action_Jump"))
  ;[1 1 1] Jump Action - AV
  (:`Started`
    (if (`self.Is Wallrunning`)
      (`self.End Wallrunning` true)
      (else
        (set `self.JumpMaxCount` 2)
        (`self.Jump`)
        ;[1 0.09412 0] Jump Audio
        (`GameplayStatics.PlaySoundAtLocation` "/Game/Audio/SFX/MediumWhoosh.MediumWhoosh" (`SceneComponent.K2_GetComponentLocation` (`self.Camera`)) (struct) 1.0 1.0 0.0 null null null null))))
  (:`Completed`
    (`self.StopJumping`)))

(event `Key|LeftShift`
  (params (Key :type "Key Structure"))
  ;[1 1 1] Shift Action (Change the players speed when shift is pressed) - AV
  (:`Pressed`
    (`self.Toggle Movement Speed`)
    (set `self.is_Sprinting` (not (`self.is_Sprinting`)))))

(event `Key|LeftControl`
  (params (Key :type "Key Structure"))
  ;[1 1 1] Ctrl Action (Allows the player to Slide) - AV
  (:`Pressed`
    (if (`self.is_Sprinting`)
      (set `SpringArmComponent.TargetOffset` (0.0 0.0 -80.0) (`self.SpringArm`))
      (`KismetSystemLibrary.K2_SetTimerDelegate` (delegate `EndSlide`) 0.75)
      ;[1 0.09412 0] Slide Audio
      (`/Engine/EditorBlueprintResources/StandardMacros.DoOnce` false :!label _label_2
        (:`Completed`
          (`GameplayStatics.PlaySoundAtLocation` "/Game/Audio/SFX/Slide.Slide" (`SceneComponent.K2_GetComponentLocation` (`self.Camera`)) (struct) 1.0 1.0 0.0 null null null null)
          (`KismetSystemLibrary.Delay` 0.75)
          (goto _label_2 :!via `Reset`))))))

(event `EndSlide`
  ;[1 1 1] Ctrl Action (Allows the player to Slide) - AV
  (set `SpringArmComponent.TargetOffset` (0.0 0.0 0.0) (`self.SpringArm`)))

(event `self.CapsuleComponent.OnComponentHit`
  (params (HitComponent :type "PrimitiveComponent Object Reference") (OtherActor :type "Actor Object Reference") (OtherComp :type "PrimitiveComponent Object Reference") (NormalImpulse :type "Vector Structure") (Hit :type "HitResult Structure (by ref)"))
  ;[1 1 1] Wallrunning - JR
  ;;[1 1 1] if not already wall running
  (if (== (`self._wallrunningWall`) null)
    ;;[1 1 1] if not wallrunnable wall
    (if (`self.ActorHasTag` OtherActor "Wallrunable")
      (if (`self.Can Wallrun`)
        (`self.Start Wallrunning` OtherActor Hit)))))

(event `EnhancedInput|/Game/Input/Actions/Action_Fire`
  (params (ActionValue :type Boolean) (ElapsedSeconds :type "Float (double-precision)") (TriggeredSeconds :type "Float (double-precision)") (InputAction :type "InputAction Object Reference" :default "/Game/Input/Actions/Action_Fire.Action_Fire"))
  (bind _camera (`self.Camera`))
  (bind _returnvalue (`SceneComponent.GetForwardVector` _camera))
  (bind _returnvalue_2 (`SceneComponent.K2_GetComponentLocation` _camera))
  ;[1 1 1] Start weapon fire when trigger is down
  (:`Started`
    (`/Game/Blueprints/WeaponHolder.TriggerDown` (`self.WeaponHolder`) _returnvalue_2 _returnvalue)
    (`GameplayStatics.PlaySoundAtLocation` "/Game/Audio/SFX/GunShot.GunShot" _returnvalue_2 (struct) 1.0 1.0 0.0 null null null null))
  (:`Canceled`
    (`/Game/Blueprints/WeaponHolder.TriggerDown` (`self.WeaponHolder`) _returnvalue_2 _returnvalue)))

(event `EnhancedInput|/Game/Input/Actions/Action_Reload`
  (params (ActionValue :type Boolean) (ElapsedSeconds :type "Float (double-precision)") (TriggeredSeconds :type "Float (double-precision)") (InputAction :type "InputAction Object Reference" :default "/Game/Input/Actions/Action_Reload.Action_Reload"))
  ;[0 0.5176 1] Reload when button is pressed
  (:`Triggered`
    (`/Game/Blueprints/WeaponHolder.ReloadPressed` (`self.WeaponHolder`))
    ;[1 0.09412 0] Reload Audio
    (`/Engine/EditorBlueprintResources/StandardMacros.DoOnce` false :!label _label_3
      (:`Completed`
        (`GameplayStatics.PlaySoundAtLocation` "/Game/Audio/SFX/RevolverReload.RevolverReload" (`SceneComponent.K2_GetComponentLocation` (`self.Camera`)) (struct) 1.0 1.0 0.0 null null null null)
        (`KismetSystemLibrary.Delay` 1.0)
        (goto _label_3 :!via `Reset`)))))

(event `self.ReceiveAnyDamage`
  (params (Damage :type "Float (single-precision)") (DamageType :type "DamageType Object Reference") (InstigatedBy :type "Controller Object Reference") (DamageCauser :type "Actor Object Reference"))
  ;[1 1 1] Health System
  (set `self.Health` (- (`self.Health`) Damage))
  (if (<= (`self.Health`) 0.0)
    (`KismetSystemLibrary.PrintString` (`KismetStringLibrary.Conv_DoubleToString` (`self.Health`)))
    (else
      (`KismetSystemLibrary.PrintString` (`KismetStringLibrary.Conv_DoubleToString` (`self.Health`))))))

(event `Key|M`
  (params (Key :type "Key Structure"))
  ;[1 1 1] Experimenting Damage (See if UI works)
  (:`Pressed`
    (`GameplayStatics.ApplyDamage` self 10.0)))

(event `self.ReceiveBeginPlay`
  ;[1 1 1] Health UI
  (bind _returnvalue (`|CreateWidget` "/Game/UI/WB_HealthSystem.WB_HealthSystem_C" (`GameplayStatics.GetPlayerController` 0)))
  (`UserWidget.AddToViewport` _returnvalue 0))

(event `EnhancedInput|/Game/Input/Actions/Action_PauseGame`
  (params (ActionValue :type Boolean) (ElapsedSeconds :type "Float (double-precision)") (TriggeredSeconds :type "Float (double-precision)") (InputAction :type "InputAction Object Reference" :default "/Game/Input/Actions/Action_PauseGame.Action_PauseGame"))
  (bind _returnvalue (`GameplayStatics.GetPlayerController` 0))
  ;[1 1 1] Pause UI
  (:`Started`
    (if (not (`self.isPauseMenuOpened?`))
      (set `self.isPauseMenuOpened?` true)
      (bind _returnvalue_2 (`|CreateWidget` "/Game/UI/WB_Pause.WB_Pause_C" _returnvalue))
      (bind _output_get (set `self.PauseMenuWB` _returnvalue_2))
      (`UserWidget.AddToViewport` (`self.PauseMenuWB`) 0)
      (`UserWidget.AddToViewport` _output_get 0)
      (`WidgetBlueprintLibrary.SetInputMode_GameAndUIEx` _returnvalue (`self.PauseMenuWB`))
      (set `PlayerController.bShowMouseCursor` true (`GameplayStatics.GetPlayerController` 0))
      (`GameplayStatics.SetGamePaused` true)
      (else
        (set `self.isPauseMenuOpened?` false)
        (`Widget.RemoveFromParent` (`self.PauseMenuWB`))
        (`GameplayStatics.SetGamePaused` false)
        (`WidgetBlueprintLibrary.SetInputMode_GameOnly` _returnvalue)
        (set `PlayerController.bShowMouseCursor` false (`GameplayStatics.GetPlayerController` 0))))))

(fn `Can Wallrun`
  (returns (Can :type Boolean))
  (bind _returnvalue (`self.K2_GetActorLocation`))
  (bind (_returnvalue_x _returnvalue_y) (`KismetMathLibrary.BreakVector` (`self.GetVelocity`)))
  (if (== (`self._wallrunningWall`) null)
    (return true)
    (else
      (bind _outhit (`KismetSystemLibrary.LineTraceSingle` _returnvalue (+ _returnvalue (* (`self._wallrunningNormal`) (-100.0 -100.0 -100.0))) "TraceTypeQuery1"))
      (return (and (and (> (`.Distance` (`GameplayStatics.BreakHitResult` _outhit)) 10.0) (== (`.HitActor` (`GameplayStatics.BreakHitResult` _outhit)) (`self._wallrunningWall`))) (`NavMovementComponent.IsFalling` (`self.CharacterMovement`)) (> (`KismetMathLibrary.Abs` (+ _returnvalue_x _returnvalue_y)) 500.0) (> (`KismetMathLibrary.Abs` (`KismetMathLibrary.Dot_VectorVector` (`SceneComponent.GetForwardVector` (`Actor.RootComponent` (`self._wallrunningWall`))) (`SceneComponent.GetForwardVector` (`self.Camera`)))) 0.5))))))

(fn `End Wallrunning`
  (params (Jump :type Boolean))
  (bind _charactermovement (`self.CharacterMovement`))
  (`MovementComponent.SetPlaneConstraintEnabled` _charactermovement false)
  (set `CharacterMovementComponent.GravityScale` 1.0 _charactermovement)
  (`SceneComponent.K2_SetRelativeRotation` :`self` (`self.Camera`))
  (if Jump
    (`self.LaunchCharacter` (* (+ (`self._wallrunningNormal`) (0.0 0.0 1.0)) (`self._wallrunningJumpForce`))))
  (set `self._wallrunningNormal` (0.0 0.0 0.0))
  (set `self._wallrunningWall` null))

(fn `Get Wall Direction`
  (returns (Direction :type Boolean))
  (return (> (`KismetMathLibrary.Dot_VectorVector` (`self._wallrunningNormal`) (`SceneComponent.GetRightVector` (`self.Camera`))) 0.0)))

(fn `Is Wallrunning`
  (returns (Is :type Boolean))
  (return (not (== (`self._wallrunningWall`) null))))

(fn `Start Wallrunning`
  (params (WallActor :type "Actor Object Reference") (WallHit :type "HitResult Structure"))
  (bind _camera (`self.Camera`))
  (bind _charactermovement (`self.CharacterMovement`))
  (bind (_returnvalue_x _returnvalue_y) (`KismetMathLibrary.BreakVector` (* (`SceneComponent.GetForwardVector` (`self.CapsuleComponent`)) (`self._wallrunningInitialForce`))))
  (if (`self.Can Wallrun`)
    (set `self._wallrunningNormal` WallHit_Normal)
    (set `self._wallrunningWall` WallActor)
    (`MovementComponent.SetPlaneConstraintEnabled` _charactermovement true)
    (`MovementComponent.SetPlaneConstraintNormal` _charactermovement WallHit_Normal)
    (if (`self.Get Wall Direction`)
      (`SceneComponent.K2_SetRelativeRotation` _camera (struct :`Roll` 10.0) false false)
      (else
        (`SceneComponent.K2_SetRelativeRotation` _camera (struct :`Roll` -10.0) false false)))
    (set `CharacterMovementComponent.GravityScale` 0.25 (`self.CharacterMovement`))
    (`self.LaunchCharacter` (`KismetMathLibrary.MakeVector` _returnvalue_x _returnvalue_y (/ (`self._wallrunningInitialForce`) 2.0)) false true)))

(fn `Toggle Movement Speed`
  ;[1 1 1] Toggle movement speed - AV
  (if (`self.is_Sprinting`)
    (bind _output_get (set `CharacterMovementComponent.MaxWalkSpeed` (`self._walkSpeed`) (`self.CharacterMovement`)))
    (set `self.MoveSpeed` _output_get)
    (else
      (bind _output_get_2 (set `CharacterMovementComponent.MaxWalkSpeed` (`self._sprintSpeed`) (`self.CharacterMovement`)))
      (set `self.MoveSpeed` _output_get_2))))

(fn `Update Wallrunning`
  (if (`self.Is Wallrunning`)
    (if (not (`self.Can Wallrun`))
      (`self.End Wallrunning` false))))

(fn `UserConstructionScript`)