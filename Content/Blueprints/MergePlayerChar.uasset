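; First-person style player character Blueprint that turns Enhanced Input actions into look, movement, firing and reload.
; Look input drives controller yaw and inverted pitch, and move input is applied along the actor's right and forward vectors.
; Fire passes camera location and forward vector to WeaponHolder.TriggerDown and plays a sound there; cancel calls TriggerDown again with zero vectors.
; Reload forwards to WeaponHolder; no jump logic is present.
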(event `self.ReceiveBeginPlay`)

(event `EnhancedInput|/Game/Input/Action_Look`
  (params (ActionValue :type "Vector2D Structure") (ElapsedSeconds :type "Float (double-precision)") (TriggeredSeconds :type "Float (double-precision)") (InputAction :type "InputAction Object Reference" :default "/Game/Input/Action_Look.Action_Look"))
  ;[1 1 1] Camera control
  (:`Triggered`
    (`self.AddControllerYawInput` ActionValue_X)
    (`self.AddControllerPitchInput` (* ActionValue_Y -1.0))))

(event `EnhancedInput|/Game/Input/Action_Move`
  (params (ActionValue :type "Vector2D Structure") (ElapsedSeconds :type "Float (double-precision)") (TriggeredSeconds :type "Float (double-precision)") (InputAction :type "InputAction Object Reference" :default "/Game/Input/Action_Move.Action_Move"))
  ;[1 1 1] Movement action and Jump action
  (:`Triggered`
    (`self.AddMovementInput` (`self.GetActorRightVector`) ActionValue_X)
    (`self.AddMovementInput` (`self.GetActorForwardVector`) ActionValue_Y)))

(event `EnhancedInput|/Game/Input/Action_Fire`
  (params (ActionValue :type Boolean) (ElapsedSeconds :type "Float (double-precision)") (TriggeredSeconds :type "Float (double-precision)") (InputAction :type "InputAction Object Reference" :default "/Game/Input/Action_Fire.Action_Fire"))
  (bind _camera (`self.Camera`))
  (bind _returnvalue (`SceneComponent.K2_GetComponentLocation` _camera))
  ;[1 1 1] Start weapon fire when trigger is down
  (:`Started`
    (`/Game/Blueprints/WeaponHolder.TriggerDown` (`self.WeaponHolder`) _returnvalue (`SceneComponent.GetForwardVector` _camera))
    (`GameplayStatics.PlaySoundAtLocation` null _returnvalue (struct) 1.0 1.0 0.0 null null null null))
  (:`Canceled`
    (`/Game/Blueprints/WeaponHolder.TriggerDown` (`self.WeaponHolder`) (0.0 0.0 0.0) (0.0 0.0 0.0))))

(event `EnhancedInput|/Game/Input/Action_Reload`
  (params (ActionValue :type Boolean) (ElapsedSeconds :type "Float (double-precision)") (TriggeredSeconds :type "Float (double-precision)") (InputAction :type "InputAction Object Reference" :default "/Game/Input/Action_Reload.Action_Reload"))
  ;[0 0.5176 1] Reload when button is pressed
  (:`Triggered`
    (`/Game/Blueprints/WeaponHolder.ReloadPressed` (`self.WeaponHolder`))))

(fn `UserConstructionScript`)