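; Weapon projectile that damages whatever it overlaps and can ricochet toward enemies a limited number of times.
; While bounces remain, an overlap flags homing and sphere-traces around the projectile, ignoring the actor just hit.
; The first "Enemy"-tagged result becomes the next target, velocity is reset from initial speed and a direction helper, and a bounce is spent.
; An overlap with no bounces left destroys it.
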(event `self._Collider.OnComponentBeginOverlap`
  (params (OverlappedComponent :type "PrimitiveComponent Object Reference") (OtherActor :type "Actor Object Reference") (OtherComp :type "PrimitiveComponent Object Reference") (OtherBodyIndex :type Integer) (bFromSweep :type Boolean) (SweepResult :type "HitResult Structure (by ref)"))
  (bind _returnvalue (`self.K2_GetActorLocation`))
  (bind __projectilemovement (`self._ProjectileMovement`))
  (bind _actorsfound (`self.ActorsFound`))
  (`GameplayStatics.ApplyDamage` OtherActor (`self.Damage`))
  (if (> (`self.BouncesLeft`) 0)
    (set `self.Homing?` true)
    (`KismetArrayLibrary.Array_Clear` _actorsfound)
    (`KismetArrayLibrary.Array_Add` _actorsfound OtherActor)
    (bind _outhits (`KismetSystemLibrary.SphereTraceMulti` _returnvalue _returnvalue 1000.0 "TraceTypeQuery3" false (`self.ActorsFound`)))
    (for _array_element _outhits
      (bind (_bblockinghit _binitialoverlap _time _distance _location _impactpoint _normal _impactnormal _physmat _hitactor) (`GameplayStatics.BreakHitResult` _array_element))
      (if (`self.ActorHasTag` _hitactor "Enemy")
        (set `self.NextTargetActor` _hitactor)
        (`KismetArrayLibrary.Array_Add` (`self.ActorsFound`) (`self.NextTargetActor`))
        (set `MovementComponent.Velocity` (* (`ProjectileMovementComponent.InitialSpeed` __projectilemovement) (`KismetMathLibrary.Normal` (- (`self.K2_GetActorLocation` (`self.NextTargetActor`)) (`self.K2_GetActorLocation`)))) __projectilemovement)
        (`/Engine/EditorBlueprintResources/StandardMacros.DecrementInt` (`self.BouncesLeft`)
          (:`  `
            (break)))))
    (else
      (`self.K2_DestroyActor`))))

(fn `UserConstructionScript`)