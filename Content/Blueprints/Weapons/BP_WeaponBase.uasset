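; Base weapon Blueprint that handles firing, ammo and reloading as either a projectile or hitscan weapon.
; Fire checks cooldown and ammo, then per bullet spawns BP_Projectile within a cone around the camera's forward or line-traces with random end offsets, applying fixed damage.
; Each shot spends one ammo and starts a cooldown timer.
; Reload instantly refills to clip capacity; CancelFire is an empty stub.
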(event `Fire`
  (params (Reticle :type "Vector Structure") (Direction :type "Vector Structure"))
  ;[1 1 1] Firing Logic, wont work if primary fire is on cooldown and tere is no ammo
  (if (`self.isPrimaryCooldown?`)
    (`KismetSystemLibrary.PrintText` "Can't shoot, weapon on cooldown")
    (elif (> (`self.availableAmmo`) 0)
      (if (`self.isProjectile?`)
        ;[1 1 1] Projectile Logic
        (for _ (range (+ (`self.bulletsPerShot`) 1))
          (bind _returnvalue (`|SpawnActorFromClass` "/Game/Blueprints/Weapons/BP_Projectile.BP_Projectile_C" (`KismetMathLibrary.MakeTransform` Reticle (`KismetMathLibrary.Conv_VectorToRotator` (`KismetMathLibrary.RandomUnitVectorInConeInDegrees` (`KismetMathLibrary.Conv_RotatorToVector` (`SceneComponent.K2_GetComponentRotation` (`/Game/Blueprints/BP_PlayerCharacter.Camera` (`self.playerREF`)))) (`self.maxWeaponSpread`)))) "Undefined" "MultiplyWithRoot" null null))
          (`GameplayStatics.PlaySoundAtLocation` null (`self.K2_GetActorLocation`) (struct) 1.0 1.0 0.0 null null _returnvalue null))
        (else
          ;[1 1 1] Base hitscan weapon logic: Trace a line by the shooting range and then apply damage to whatever it hit.
          (for _ (range (+ (`self.bulletsPerShot`) 1))
            (bind _outhit (`KismetSystemLibrary.LineTraceSingle` :`Start` Reticle :`End` (`KismetMathLibrary.MakeVector` (+ (.x (+ Reticle (* Direction (`self.fireRange`)))) (`KismetMathLibrary.RandomFloatInRange` (`self.minWeaponSpread`) (`self.maxWeaponSpread`))) (+ (.y (+ Reticle (* Direction (`self.fireRange`)))) (`KismetMathLibrary.RandomFloatInRange` (`self.minWeaponSpread`) (`self.maxWeaponSpread`))) (+ (.z (+ Reticle (* Direction (`self.fireRange`)))) (`KismetMathLibrary.RandomFloatInRange` (`self.minWeaponSpread`) (`self.maxWeaponSpread`)))) :`TraceChannel` "TraceTypeQuery1" :`DrawDebugType` "ForDuration" :`DrawTime` 1.0))
            (`GameplayStatics.ApplyDamage` (`.HitActor` (`GameplayStatics.BreakHitResult` _outhit)) 10.0)
            (`GameplayStatics.PlaySound2D` null 1.0 1.0 0.0 null null))))
      ;[1 1 1] Removing ammo and Cooldown TImer
      (set `self.availableAmmo` (- (`self.availableAmmo`) 1))
      (set `self.isPrimaryCooldown?` true)
      (`KismetSystemLibrary.K2_SetTimerDelegate` (delegate `Reset Primary Timer`) (`self.primaryFireRate`))
      (`KismetSystemLibrary.PrintString` (`KismetStringLibrary.Conv_IntToString` (`self.availableAmmo`)))
      (else
        (`KismetSystemLibrary.PrintString` "Out of ammo, Reload")))))

(event `Reset Primary Timer`
  ;[1 1 1] Removing ammo and Cooldown TImer
  (set `self.isPrimaryCooldown?` false))

(event `Reload`
  ;[0 0.5176 1] Reload Logic
  (set `self.availableAmmo` (`self.clipCapacity`))
  (`GameplayStatics.PlaySound2D` null 1.0 1.0 0.0 null null))

(event `Cancel Fire`)

(fn `UserConstructionScript`)