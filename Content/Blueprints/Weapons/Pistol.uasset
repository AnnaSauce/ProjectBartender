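; Pistol weapon Blueprint that fires a single hitscan shot and plays revolver fire and reload animations.
; Firing and reloading temporarily link animation layers on the mesh, using fixed delays before unlinking.
; The shot traces only after the fire delay, then passes critical-hit status to actors implementing BPI_Hitbox.
; Reload calls the parent logic first; disconnected range, projectile and spread-fire nodes remain unused.
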(event `self.OnFire`
  (bind __mesh (`self._Mesh`))
  (`SkeletalMeshComponent.LinkAnimClassLayers` __mesh "/Game/Animation/ABP_RevolverFire.ABP_RevolverFire_C")
  (`KismetSystemLibrary.Delay` 0.5)
  (`SkeletalMeshComponent.UnlinkAnimClassLayers` __mesh "/Game/Animation/ABP_RevolverFire.ABP_RevolverFire_C")
  (bind (_criticalhit _actorhit) (`self.Fire_Hitscan_Single`))
  (if (`KismetSystemLibrary.DoesImplementInterface` _actorhit "/Game/Blueprints/BPI_Hitbox.BPI_Hitbox_C")
    (message `/Game/Blueprints/BPI_Hitbox.ManageCriticalHit` _actorhit _criticalhit)))

(event `self.Reload`
  (`parent.Reload`)
  (`SkeletalMeshComponent.LinkAnimClassLayers` (`self._Mesh`) "/Game/Animation/ABP_RevolverReload.ABP_RevolverReload_C")
  (`KismetSystemLibrary.Delay` 1.1)
  (`SkeletalMeshComponent.UnlinkAnimClassLayers` (`self._Mesh`) "/Game/Animation/ABP_RevolverReload.ABP_RevolverReload_C"))

(fn `UserConstructionScript`)