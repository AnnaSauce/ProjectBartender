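; WeaponHolderFreddie is a weapon-holder component that relays trigger input to a weapon.
; On BeginPlay it spawns WeaponToSpawn at its relative transform under the same owner, then sets Weapon to None, not the spawned actor, before calling attach-to-self on it.
; TriggerDown passes reticle and direction to the weapon's Fire and TriggerUp calls StopFiring, both only when Weapon is valid.
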(event `self.ReceiveBeginPlay`
  (bind _returnvalue (`|SpawnActorFromClass` (`.WeaponToSpawn` (`self.WeaponToSpawn`)) (`self.GetRelativeTransform`) "AlwaysSpawn" "MultiplyWithRoot" (`self.GetOwner`) null))
  (bind (_output_get _output_get_2) (set `self.Weapon` null _returnvalue))
  (`Actor.K2_AttachToComponent` _output_get_2 self "None" "KeepRelative" "KeepRelative" "KeepRelative" true))

(event `TriggerDown`
  (params (Reticle :type "Vector Structure") (Direction :type "Vector Structure"))
  (bind (_weapon _weapon_2) (`self.Weapon`))
  ;[1 1 1] If there is a weapon, shoot it
  (`/Engine/EditorBlueprintResources/StandardMacros.IsValid` _weapon_2
    (:`Is Valid`
      (`self.Fire` _weapon_2 Reticle Direction))))

(event `TriggerUp`
  (bind (_weapon _weapon_2) (`self.Weapon`))
  ;[1 1 1] If there is a weapon, shoot it
  (`/Engine/EditorBlueprintResources/StandardMacros.IsValid` _weapon_2
    (:`Is Valid`
      (`self.StopFiring` _weapon_2))))