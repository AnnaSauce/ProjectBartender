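; Projectile Blueprint that damages what it hits and attempts to ricochet toward nearby actors tagged Enemy.
; On hit, it loops over the ricochet count, damaging ignore-list entries and sphere-tracing around them to set a homing target.
; The projectile is destroyed right after the loop, so homing never plays out.
; Only the first hit actor joins the list, as the node adding traced actors is unconnected, leaving later iterations without valid entries.
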(event `self._Collider.OnComponentHit`
  (params (HitComponent :type "PrimitiveComponent Object Reference") (OtherActor :type "Actor Object Reference") (OtherComp :type "PrimitiveComponent Object Reference") (NormalImpulse :type "Vector Structure") (Hit :type "HitResult Structure (by ref)"))
  (bind _actorstoignore (`self.ActorsToIgnore`))
  (bind __projectilemovement (`self._ProjectileMovement`))
  (`KismetArrayLibrary.Array_Clear` _actorstoignore)
  (`KismetArrayLibrary.Array_Add` _actorstoignore OtherActor)
  (for _index (range (+ (`self.TimesToRicochet`) 1))
    (bind _output (`|GetArrayItem` (`self.ActorsToIgnore`) _index))
    (`GameplayStatics.ApplyDamage` _output 20.0)
    (bind _returnvalue (`self.K2_GetActorLocation` _output))
    (bind _outhit (`KismetSystemLibrary.SphereTraceSingle` _returnvalue _returnvalue 600.0 "TraceTypeQuery3" false (`self.ActorsToIgnore`) "Persistent"))
    (bind (_bblockinghit _binitialoverlap _time _distance _location _impactpoint _normal _impactnormal _physmat _hitactor _hitcomponent) (`GameplayStatics.BreakHitResult` _outhit))
    (bind _returnvalue_2 (`self.ActorHasTag` _hitactor "Enemy"))
    (if _returnvalue_2
      (set `ProjectileMovementComponent.bIsHomingProjectile` _returnvalue_2 __projectilemovement)
      (set `ProjectileMovementComponent.HomingTargetComponent` _hitcomponent __projectilemovement)))
  (`self.K2_DestroyActor`))

(fn `UserConstructionScript`)