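; MergeWeapBase is a weapon Blueprint, apparently a base class, that handles firing, ammo and reloading.
; Fire checks cooldown and ammo, then either spawns BP_Projectile along the player camera's rotation or runs a debug-drawn hitscan trace with random endpoint spread and fixed damage.
; Each shot spends one round and starts a timer that clears the cooldown at the fire rate.
; Reload instantly refills ammo, and CancelFire is an empty stub.
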(event `Fire`
  (params (Reticle :type "Vector Structure") (Direction :type "Vector Structure"))
  (bind _returnvalue (`KismetMathLibrary.RandomFloatInRange` (`self.minWeaponSpread`) (`self.maxWeaponSpread`)))
  ;[1 1 1] Firing Logic, wont work if primary fire is on cooldown and tere is no ammo
  (if (`self.isPrimaryCooldown?`)
    (`KismetSystemLibrary.PrintText` "Can't shoot, weapon on cooldown")
    (elif (> (`self.currentAmmo`) 0)
      (if (`self.isProjectile?`)
        ;[1 1 1] Projectile Logic
        (bind _returnvalue_2 (`|SpawnActorFromClass` "/Game/Blueprints/Weapons/BP_Projectile.BP_Projectile_C" (`KismetMathLibrary.MakeTransform` Reticle (`SceneComponent.K2_GetComponentRotation` (`/Game/Blueprints/BP_PlayerCharacter.Camera` (`self.playerREF`)))) "Undefined" "MultiplyWithRoot" null null))
        (`GameplayStatics.PlaySoundAtLocation` null (`self.K2_GetActorLocation`) (struct) 1.0 1.0 0.0 null null _returnvalue_2 null)
        (else
          ;[1 1 1] Base hitscan weapon logic: Trace a line by the shooting range and then apply damage to whatever it hit.
          (bind _outhit (`KismetSystemLibrary.LineTraceSingle` :`Start` Reticle :`End` (`KismetMathLibrary.MakeVector` (+ (.x (+ Reticle (* Direction (`self.Fire Range`)))) _returnvalue) (+ (.y (+ Reticle (* Direction (`self.Fire Range`)))) _returnvalue) (+ (.z (+ Reticle (* Direction (`self.Fire Range`)))) _returnvalue)) :`TraceChannel` "TraceTypeQuery1" :`DrawDebugType` "ForDuration" :`DrawTime` 1.0))
          (`GameplayStatics.ApplyDamage` (`.HitActor` (`GameplayStatics.BreakHitResult` _outhit)) 10.0)
          (`GameplayStatics.PlaySound2D` null 1.0 1.0 0.0 null null)))
      ;[1 1 1] Removing ammo and Cooldown TImer
      (set `self.currentAmmo` (- (`self.currentAmmo`) 1))
      (set `self.isPrimaryCooldown?` true)
      (`KismetSystemLibrary.K2_SetTimerDelegate` (delegate `Reset Primary Timer`) (`self.primaryFireRate`))
      (`KismetSystemLibrary.PrintString` (`KismetStringLibrary.Conv_IntToString` (`self.currentAmmo`)))
      (else
        (`KismetSystemLibrary.PrintString` "Out of ammo, Reload")))))

(event `Reset Primary Timer`
  ;[1 1 1] Removing ammo and Cooldown TImer
  (set `self.isPrimaryCooldown?` false))

(event `Reload`
  ;[0 0.5176 1] Reload Logic
  (set `self.currentAmmo` (`self.maxAmmo`))
  (`GameplayStatics.PlaySound2D` null 1.0 1.0 0.0 null null))

(event `Cancel Fire`)

(fn `UserConstructionScript`)