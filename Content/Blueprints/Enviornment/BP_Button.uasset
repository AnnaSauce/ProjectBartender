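; BP_Button is an environment button that triggers car crusher traps when it takes any damage.
; A ButtonPressed timeline lerps the button mesh's Z position to animate the press.
; Behind a DoOnce, it searches all BP_CarCrusher actors and calls ActivateTrap on those whose ID matches its ButtonID.
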(event `self.ReceiveAnyDamage`
  (params (Damage :type "Float (single-precision)") (DamageType :type "DamageType Object Reference") (InstigatedBy :type "Controller Object Reference") (DamageCauser :type "Actor Object Reference"))
  ;[1 1 1] Button Pressing
  (bind (_direction _height) (`Timeline|Button Pressed`)
    (:`Update`
      (`SceneComponent.K2_SetRelativeLocation` (`self.SM_Button`) (`KismetMathLibrary.MakeVector` 0.0 0.0 (`KismetMathLibrary.Lerp` 1.0 -12.0 _height)) false false)
      (`/Engine/EditorBlueprintResources/StandardMacros.DoOnce` false
        (:`Completed`
          ;[1 1 1] This iterates through each Car Crusher object in the scene to find one that shares the same ID Value as the button
          (bind _outactors (`GameplayStatics.GetAllActorsOfClass` "/Game/Blueprints/Enviornment/BP_CarCrusher.BP_CarCrusher_C"))
          (for _array_element _outactors
            (if (== (`/Game/Blueprints/Enviornment/BP_CarCrusher.ID` _array_element) (`self.ButtonID`))
              (`/Game/Blueprints/Enviornment/BP_CarCrusher.Activate Trap` _array_element))))))))

(fn `UserConstructionScript`)