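; BP_HangingCar is an environmental hazard: a suspended car that drops when it takes damage.
; On BeginPlay the SMCar mesh's gravity follows the IsFalling flag, and any damage sets the flag true and enables gravity.
; The HurtBox overlap applies the Damage value to the overlapping actor, but only while IsFalling is set, which is never cleared in this graph.
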(event `self.ReceiveBeginPlay`
  ;[1 1 1] On Start
  (`PrimitiveComponent.SetEnableGravity` (`self.SM_Car`) (`self.isFalling?`)))

(event `self.ReceiveAnyDamage`
  (params (Damage :type "Float (single-precision)") (DamageType :type "DamageType Object Reference") (InstigatedBy :type "Controller Object Reference") (DamageCauser :type "Actor Object Reference"))
  ;[0 1 0.2395] When Shot, activate gravity
  (bind _output_get (set `self.isFalling?` true))
  (`PrimitiveComponent.SetEnableGravity` (`self.SM_Car`) _output_get))

(event `self.HurtBox.OnComponentBeginOverlap`
  (params (OverlappedComponent :type "PrimitiveComponent Object Reference") (OtherActor :type "Actor Object Reference") (OtherComp :type "PrimitiveComponent Object Reference") (OtherBodyIndex :type Integer) (bFromSweep :type Boolean) (SweepResult :type "HitResult Structure (by ref)"))
  ;[1 0 0.0258] Damage Logic
  (if (`self.isFalling?`)
    (`GameplayStatics.ApplyDamage` OtherActor (`self.damage`))))

(fn `UserConstructionScript`)