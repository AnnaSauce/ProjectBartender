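; BP_CarCrusher is a crusher trap with two sides that endlessly open and close once ActivateTrap is triggered.
; Two timelines lerp the side meshes apart and together, each calling ActivateTrap again when finished, with a player camera shake on every close.
; Left and right box overlaps maintain HitCount; while it is at least two, Tick applies damage every frame to the actor from LeftBox's begin overlap.
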(event `self.ReceiveTick`
  (params (DeltaSeconds :type "Float (single-precision)"))
  ;[1 0 0] Damage Logic
  (if (>= (`self.hitCount`) 2)
    (`GameplayStatics.ApplyDamage` (stale `self.LeftBox.OnComponentBeginOverlap` OtherActor) (`self.damage`))))

(event `self.LeftBox.OnComponentBeginOverlap`
  (params (OverlappedComponent :type "PrimitiveComponent Object Reference") (OtherActor :type "Actor Object Reference") (OtherComp :type "PrimitiveComponent Object Reference") (OtherBodyIndex :type Integer) (bFromSweep :type Boolean) (SweepResult :type "HitResult Structure (by ref)"))
  ;[1 1 1] Collision Logic
  (set `self.hitCount` (+ (`self.hitCount`) 1)))

(event `Activate Trap`
  (if (`self.isClosed?`)
    ;[1 1 1] Opening Crusher
    (bind (_direction _opening_animation) (`Timeline|Timeline` :!via `PlayFromStart`)
      (:`Update`
        (`SceneComponent.K2_SetRelativeLocation` (`self.SM_LeftSide`) (`KismetMathLibrary.VLerp` (-12.0 0.0 0.0) (-50.0 0.0 0.0) _opening_animation) false false)
        (`SceneComponent.K2_SetRelativeLocation` (`self.SM_RightSide`) (`KismetMathLibrary.VLerp` (12.0 0.0 0.0) (50.0 0.0 0.0) _opening_animation) false false))
      (:`Finished`
        (set `self.isClosed?` false)
        (`self.Activate Trap`)))
    (else
      ;[1 1 1] Closing Crusher
      (bind (_direction_2 _closing_animation) (`Timeline|Crusher Closing Animation` :!via `PlayFromStart`)
        (:`Update`
          (`SceneComponent.K2_SetRelativeLocation` (`self.SM_LeftSide`) (`KismetMathLibrary.VLerp` (-50.0 0.0 0.0) (-12.0 0.0 0.0) _closing_animation) false false)
          (`SceneComponent.K2_SetRelativeLocation` (`self.SM_RightSide`) (`KismetMathLibrary.VLerp` (50.0 0.0 0.0) (12.0 0.0 0.0) _closing_animation) false false))
        (:`Finished`
          (set `self.isClosed?` true)
          (`PlayerCameraManager.StartCameraShake` :`self` (`GameplayStatics.GetPlayerCameraManager` 0) :`ShakeClass` "/Game/Blueprints/Camera_Shake/BP_CarCrusherShake.BP_CarCrusherShake_C" :`PlaySpace` "World")
          (`self.Activate Trap`))))))

(event `self.RightBox.OnComponentBeginOverlap`
  (params (OverlappedComponent :type "PrimitiveComponent Object Reference") (OtherActor :type "Actor Object Reference") (OtherComp :type "PrimitiveComponent Object Reference") (OtherBodyIndex :type Integer) (bFromSweep :type Boolean) (SweepResult :type "HitResult Structure (by ref)"))
  ;[1 1 1] Collision Logic
  (set `self.hitCount` (+ (`self.hitCount`) 1)))

(event `self.LeftBox.OnComponentEndOverlap`
  (params (OverlappedComponent :type "PrimitiveComponent Object Reference") (OtherActor :type "Actor Object Reference") (OtherComp :type "PrimitiveComponent Object Reference") (OtherBodyIndex :type Integer))
  ;[1 1 1] End Collision Logic
  (set `self.hitCount` (- (`self.hitCount`) 1)))

(event `self.RightBox.OnComponentEndOverlap`
  (params (OverlappedComponent :type "PrimitiveComponent Object Reference") (OtherActor :type "Actor Object Reference") (OtherComp :type "PrimitiveComponent Object Reference") (OtherBodyIndex :type Integer))
  ;[1 1 1] End Collision Logic
  (set `self.hitCount` (- (`self.hitCount`) 1)))

(fn `UserConstructionScript`)