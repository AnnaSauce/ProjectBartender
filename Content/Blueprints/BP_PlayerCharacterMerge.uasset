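; First-person player character Blueprint with double jump, sprint, slide, wallrunning, grapple swinging, weapon input, health, HUD and pause menu.
; Tick updates wallrunning, started by hits on tagged walls using a plane constraint and low gravity, and grappling.
; An overlap collider gathers grapple points, and swinging clamps rope length by projecting out radial velocity.
; A looping timer decays slide speed, WeaponHolder handles weapons, and damage only lowers and prints Health.
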(event `self.ReceiveTick`
  (params (DeltaSeconds :type "Float (single-precision)"))
  ;[1 0 0.07548] Tick
  (`self.Update Wallrunning`)
  (`self.UpdateGrapple`))

(event `EnhancedInput|/Game/Input/Actions/Action_Look`
  (params (ActionValue :type "Vector2D Structure") (ElapsedSeconds :type "Float (double-precision)") (TriggeredSeconds :type "Float (double-precision)") (InputAction :type "InputAction Object Reference" :default "/Game/Input/Actions/Action_Look.Action_Look"))
  ;[1 1 1] Camera Action - JR
  (:`Triggered`
    (`self.AddControllerYawInput` ActionValue_X)
    (`self.AddControllerPitchInput` (* ActionValue_Y -1.0))))

(event `EnhancedInput|/Game/Input/Actions/Action_Move`
  (params (ActionValue :type "Vector2D Structure") (ElapsedSeconds :type "Float (double-precision)") (TriggeredSeconds :type "Float (double-precision)") (InputAction :type "InputAction Object Reference" :default "/Game/Input/Actions/Action_Move.Action_Move"))
  ;[1 1 1] Movement Action - AV
  (:`Triggered`
    (`self.AddMovementInput` (`self.GetActorRightVector`) ActionValue_X)
    (`self.AddMovementInput` (`self.GetActorForwardVector`) ActionValue_Y)
    ;[1 0.09393 0] Walk/Run Cycle Audio
    (`/Engine/EditorBlueprintResources/StandardMacros.DoOnce` false :!label _label
      (:`Completed`
        (`GameplayStatics.PlaySoundAtLocation` "/Game/Audio/SFX/StepSound.StepSound" (`SceneComponent.K2_GetComponentLocation` (`self.Camera`)) (struct) 1.0 1.0 0.0 null null null null)
        (if (`self.is_Sprinting`)
          (`KismetSystemLibrary.Delay` 0.25)
          (goto _label :!via `Reset`)
          (else
            (`KismetSystemLibrary.Delay` 0.5)
            (goto _label :!via `Reset`)))))))

(event `EnhancedInput|/Game/Input/Actions/Action_Jump`
  (params (ActionValue :type Boolean) (ElapsedSeconds :type "Float (double-precision)") (TriggeredSeconds :type "Float (double-precision)") (InputAction :type "InputAction Object Reference" :default "/Game/Input/Actions/Action_Jump.Action_Jump"))
  ;[1 1 1] Jump Action - AV
  (:`Started`
    (if (`self.Is Wallrunning`)
      (`self.End Wallrunning` true)
      (else
        (set `self.JumpMaxCount` 2)
        (`self.Jump`)
        ;[1 0.09412 0] Jump Audio
        (`GameplayStatics.PlaySoundAtLocation` "/Game/Audio/SFX/MediumWhoosh.MediumWhoosh" (`SceneComponent.K2_GetComponentLocation` (`self.Camera`)) (struct) 1.0 1.0 0.0 null null null null))))
  (:`Completed`
    (`self.StopJumping`)))

(event `Key|LeftShift`
  (params (Key :type "Key Structure"))
  ;[1 1 1] Shift Action (Change the players speed when shift is pressed) - AV
  (:`Pressed`
    (`self.Toggle Movement Speed`)
    (set `self.is_Sprinting` (not (`self.is_Sprinting`)))))

(event `Key|LeftControl`
  (params (Key :type "Key Structure"))
  ;[1 1 1] Ctrl Action (Allows the player to Slide) - AV
  (:`Pressed`
    (if true
      (set `self._isSliding` true)
      (`self.BeginSlide`)
      ;[1 0.09412 0] Slide Audio
      (`GameplayStatics.PlaySoundAtLocation` "/Game/Audio/SFX/Slide.Slide" (`SceneComponent.K2_GetComponentLocation` (`self.Camera`)) (struct) 1.0 1.0 0.0 null null null null)
      (bind _returnvalue (`KismetSystemLibrary.K2_SetTimerDelegate` (delegate `Slide`) 0.1 true))
      (else
        (set `self._isCrouching` (== (`self._isCrouching`) false))
        (`self.Toggle Crouch`))))
  (:`Released`
    (if (`self._isSliding`)
      (`self.EndSlide`))))

(event `Key|LeftControl`
  (params (Key :type "Key Structure"))
  ;[1 1 1] Ctrl Action (Allows the player to Slide) - AV
)

(event `Slide`
  ;[1 1 1] Ctrl Action (Allows the player to Slide) - AV
  (if (>= (`KismetMathLibrary.VSize` (`self.GetVelocity`)) 200.0)
    (if (`self._isSliding`)
      (set `CharacterMovementComponent.MaxWalkSpeed` (* 0.9 (`KismetMathLibrary.VSize` (`self.GetVelocity`))) (`self.CharacterMovement`))
      (else
        (`self.EndSlide` :!label _label_2)
        (`KismetSystemLibrary.K2_PauseTimerHandle` (stale `Key|LeftControl` _returnvalue))))
    (else
      (goto _label_2))))

(event `self.CapsuleComponent.OnComponentHit`
  (params (HitComponent :type "PrimitiveComponent Object Reference") (OtherActor :type "Actor Object Reference") (OtherComp :type "PrimitiveComponent Object Reference") (NormalImpulse :type "Vector Structure") (Hit :type "HitResult Structure (by ref)"))
  ;[1 1 1] Wallrunning - JR
  ;;[1 1 1] if not already wall running
  (if (== (`self._wallrunningWall`) null)
    ;;[1 1 1] if not wallrunnable wall
    (if (`self.ActorHasTag` OtherActor "Wallrunable")
      (`self.Start Wallrunning` OtherActor Hit))))

(event `EnhancedInput|/Game/Input/Actions/Action_Fire`
  (params (ActionValue :type Boolean) (ElapsedSeconds :type "Float (double-precision)") (TriggeredSeconds :type "Float (double-precision)") (InputAction :type "InputAction Object Reference" :default "/Game/Input/Actions/Action_Fire.Action_Fire"))
  (bind _camera (`self.Camera`))
  (bind _returnvalue (`SceneComponent.GetForwardVector` _camera))
  (bind _returnvalue_2 (`SceneComponent.K2_GetComponentLocation` _camera))
  ;[1 1 1] Start weapon fire when trigger is down
  (:`Started`
    (`/Game/Blueprints/WeaponHolder.TriggerDown` (`self.WeaponHolder`) _returnvalue_2 _returnvalue))
  (:`Canceled`
    (`/Game/Blueprints/WeaponHolder.TriggerDown` (`self.WeaponHolder`) _returnvalue_2 _returnvalue)))

(event `EnhancedInput|/Game/Input/Actions/Action_Reload`
  (params (ActionValue :type Boolean) (ElapsedSeconds :type "Float (double-precision)") (TriggeredSeconds :type "Float (double-precision)") (InputAction :type "InputAction Object Reference" :default "/Game/Input/Actions/Action_Reload.Action_Reload"))
  ;[0 0.5176 1] Reload when button is pressed
  (:`Triggered`
    (`/Game/Blueprints/WeaponHolder.ReloadPressed` (`self.WeaponHolder`))))

(event `EnhancedInput|/Game/Input/Actions/Action_Switching`
  (params (ActionValue :type "Float (double-precision)") (ElapsedSeconds :type "Float (double-precision)") (TriggeredSeconds :type "Float (double-precision)") (InputAction :type "InputAction Object Reference" :default "/Game/Input/Actions/Action_Switching.Action_Switching"))
  ;[1 1 1] Weapon Switching
  (:`Triggered`
    (`/Game/Blueprints/WeaponHolder.Switch Weapon` (`self.WeaponHolder`) ActionValue)))

(event `self.ReceiveAnyDamage`
  (params (Damage :type "Float (single-precision)") (DamageType :type "DamageType Object Reference") (InstigatedBy :type "Controller Object Reference") (DamageCauser :type "Actor Object Reference"))
  ;[1 1 1] Health System
  (set `self.Health` (- (`self.Health`) Damage))
  (if (<= (`self.Health`) 0.0)
    (`KismetSystemLibrary.PrintString` (`KismetStringLibrary.Conv_DoubleToString` (`self.Health`)))
    (else
      (`KismetSystemLibrary.PrintString` (`KismetStringLibrary.Conv_DoubleToString` (`self.Health`))))))

(event `Key|M`
  (params (Key :type "Key Structure"))
  ;[1 1 1] Experimenting Damage (See if UI works)
  (:`Pressed`
    (`GameplayStatics.ApplyDamage` self 10.0)))

(event `self.ReceiveBeginPlay`
  ;[1 1 1] Health UI
  (bind _returnvalue (`|CreateWidget` "/Game/UI/WB_HUD.WB_HUD_C" (`GameplayStatics.GetPlayerController` 0)))
  (`UserWidget.AddToViewport` _returnvalue 0))

(event `EnhancedInput|/Game/Input/Actions/Action_PauseGame`
  (params (ActionValue :type Boolean) (ElapsedSeconds :type "Float (double-precision)") (TriggeredSeconds :type "Float (double-precision)") (InputAction :type "InputAction Object Reference" :default "/Game/Input/Actions/Action_PauseGame.Action_PauseGame"))
  (bind _returnvalue (`GameplayStatics.GetPlayerController` 0))
  ;[1 1 1] Pause UI
  (:`Started`
    (if (not (`self.isPauseMenuOpened?`))
      (set `self.isPauseMenuOpened?` true)
      (bind _returnvalue_2 (`|CreateWidget` "/Game/UI/WB_Pause.WB_Pause_C" _returnvalue))
      (bind _output_get (set `self.PauseMenuWB` _returnvalue_2))
      (`UserWidget.AddToViewport` (`self.PauseMenuWB`) 0)
      (`UserWidget.AddToViewport` _output_get 0)
      (`WidgetBlueprintLibrary.SetInputMode_GameAndUIEx` _returnvalue (`self.PauseMenuWB`))
      (set `PlayerController.bShowMouseCursor` true (`GameplayStatics.GetPlayerController` 0))
      (`GameplayStatics.SetGamePaused` true)
      (else
        (set `self.isPauseMenuOpened?` false)
        (`Widget.RemoveFromParent` (`self.PauseMenuWB`))
        (`GameplayStatics.SetGamePaused` false)
        (`WidgetBlueprintLibrary.SetInputMode_GameOnly` _returnvalue)
        (set `PlayerController.bShowMouseCursor` false (`GameplayStatics.GetPlayerController` 0))))))

(event `self.GrappleCollider.OnComponentBeginOverlap`
  (params (OverlappedComponent :type "PrimitiveComponent Object Reference") (OtherActor :type "Actor Object Reference") (OtherComp :type "PrimitiveComponent Object Reference") (OtherBodyIndex :type Integer) (bFromSweep :type Boolean) (SweepResult :type "HitResult Structure (by ref)"))
  ;[1 1 1] Grapple Collider - JR
  (if (== (`GameplayStatics.GetObjectClass` OtherActor) "/Game/Blueprints/Enviornment/BP_GrapplePoint.BP_GrapplePoint_C")
    (bind _asbp_grapple_point (cast `/Game/Blueprints/Enviornment/BP_GrapplePoint` OtherActor))
    (`/Game/Blueprints/Enviornment/BP_GrapplePoint.SetActive` _asbp_grapple_point true)
    (`KismetArrayLibrary.Array_Add` (`self._grapplePoints`) _asbp_grapple_point)))

(event `self.GrappleCollider.OnComponentEndOverlap`
  (params (OverlappedComponent :type "PrimitiveComponent Object Reference") (OtherActor :type "Actor Object Reference") (OtherComp :type "PrimitiveComponent Object Reference") (OtherBodyIndex :type Integer))
  ;[1 1 1] Grapple Collider - JR
  (if (== (`GameplayStatics.GetObjectClass` OtherActor) "/Game/Blueprints/Enviornment/BP_GrapplePoint.BP_GrapplePoint_C")
    (bind _asbp_grapple_point (cast `/Game/Blueprints/Enviornment/BP_GrapplePoint` OtherActor))
    (`/Game/Blueprints/Enviornment/BP_GrapplePoint.SetActive` _asbp_grapple_point false)
    (`KismetArrayLibrary.Array_RemoveItem` (`self._grapplePoints`) _asbp_grapple_point)))

(event `EnhancedInput|/Game/Input/Actions/Action_Grapple`
  (params (ActionValue :type Boolean) (ElapsedSeconds :type "Float (double-precision)") (TriggeredSeconds :type "Float (double-precision)") (InputAction :type "InputAction Object Reference" :default "/Game/Input/Actions/Action_Grapple.Action_Grapple"))
  (bind _returnvalue (`self.K2_GetActorLocation`))
  (bind (_grapplepoint _can) (`self.CanGrapple`))
  ;[1 1 1] Grapple Input - JR
  (:`Started`
    (if _can
      (set `self._grappling` _grapplepoint)
      (bind _returnvalue_2 (`|SpawnActorFromClass` "/Script/CableComponent.CableActor" (`self.GetTransform`) "Undefined" "MultiplyWithRoot" null null))
      (set `self._grappleCable` _returnvalue_2)
      (`CableComponent.SetAttachEndTo` (`CableActor.CableComponent` _returnvalue_2) _grapplepoint "None" "None")
      (set `self._grappleStartVelocity` (`self.GetVelocity`))
      (set `self._grappleStartPosition` _returnvalue)
      (set `self._grappleDistance` (`KismetMathLibrary.VSize` (- _returnvalue (`self.K2_GetActorLocation` (`self._grappling`)))))))
  (:`Canceled`
    (`self.EndGrapple` :!label _label_3))
  (:`Completed`
    (goto _label_3)))

(fn `BeginSlide`
  (`CapsuleComponent.SetCapsuleHalfHeight` (`self.CapsuleComponent`) 40.0 true))

(fn `Can Wallrun`
  (returns (Can :type Boolean))
  (bind _returnvalue (`self.K2_GetActorLocation`))
  (bind (_returnvalue_x _returnvalue_y) (`KismetMathLibrary.BreakVector` (`self.GetVelocity`)))
  (bind __wallrunningwall (`self._wallrunningWall`))
  (bind _outhit (`KismetSystemLibrary.LineTraceSingle` _returnvalue (+ _returnvalue (* (`self._wallrunningNormal`) (-100.0 -100.0 -100.0))) "TraceTypeQuery1"))
  (return (and (and (<= (`.Distance` (`GameplayStatics.BreakHitResult` _outhit)) 50.0) (== (`.HitActor` (`GameplayStatics.BreakHitResult` _outhit)) __wallrunningwall)) (`NavMovementComponent.IsFalling` (`self.CharacterMovement`)) (>= (`KismetMathLibrary.Abs` (+ _returnvalue_x _returnvalue_y)) (/ (`self._walkSpeed`) 2.0)) (> (`KismetMathLibrary.Abs` (`KismetMathLibrary.Dot_VectorVector` (`SceneComponent.GetForwardVector` (`Actor.RootComponent` __wallrunningwall)) (`SceneComponent.GetForwardVector` (`self.Camera`)))) 0.5))))

(fn `CanGrapple`
  (returns (GrapplePoint :type "/Game/Blueprints/Enviornment/BP_GrapplePoint Object Reference") (Can :type Boolean))
  (bind __grapplepoints (`self._grapplePoints`))
  (if (or (!= (`self._grappling`) null) (> (`KismetArrayLibrary.Array_Length` __grapplepoints) 0) (`NavMovementComponent.IsFalling` (`self.CharacterMovement`)))
    (for _array_element __grapplepoints
      (if (>= (`KismetMathLibrary.Dot_VectorVector` (`KismetMathLibrary.Normal` (- (`self.K2_GetActorLocation` _array_element) (`self.K2_GetActorLocation`))) (`SceneComponent.GetForwardVector` (`self.Camera`))) 0.75)
        (return _array_element true)))
    (return null false)
    (else
      (return null false))))

(fn `End Wallrunning`
  (params (Jump :type Boolean))
  (bind _charactermovement (`self.CharacterMovement`))
  (`MovementComponent.SetPlaneConstraintEnabled` _charactermovement false)
  (set `CharacterMovementComponent.GravityScale` 1.0 _charactermovement)
  (`SceneComponent.K2_SetRelativeRotation` :`self` (`self.Camera`))
  (if Jump
    (`self.LaunchCharacter` (* (+ (`self._wallrunningNormal`) (0.0 0.0 1.0)) (`self._wallrunningJumpForce`))))
  (set `self._wallrunningNormal` (0.0 0.0 0.0))
  (set `self._wallrunningWall` null))

(fn `EndGrapple`
  (bind __grapplecable (`self._grappleCable`))
  (set `self._grappling` null)
  (`/Engine/EditorBlueprintResources/StandardMacros.IsValid` __grapplecable
    (:`Is Valid`
      (`self.K2_DestroyActor` __grapplecable))))

(fn `EndSlide`
  (set `self._isSliding` false)
  (`CapsuleComponent.SetCapsuleHalfHeight` (`self.CapsuleComponent`) 88.0 true)
  (set `CharacterMovementComponent.MaxWalkSpeed` (`self._sprintSpeed`) (`self.CharacterMovement`)))

(fn `Get Wall Direction`
  (returns (Direction :type Boolean))
  (return (> (`KismetMathLibrary.Dot_VectorVector` (`self._wallrunningNormal`) (`SceneComponent.GetRightVector` (`self.Camera`))) 0.0)))

(fn `Is Wallrunning`
  (returns (Is :type Boolean))
  (return (not (== (`self._wallrunningWall`) null))))

(fn `Start Wallrunning`
  (params (WallActor :type "Actor Object Reference") (WallHit :type "HitResult Structure"))
  (bind _charactermovement (`self.CharacterMovement`))
  (bind _camera (`self.Camera`))
  (bind (_returnvalue_x _returnvalue_y) (`KismetMathLibrary.BreakVector` (* (`SceneComponent.GetForwardVector` (`self.CapsuleComponent`)) (`self._wallrunningInitialForce`))))
  (set `self._wallrunningNormal` WallHit_Normal)
  (set `self._wallrunningWall` WallActor)
  (if (and (< (`KismetMathLibrary.Abs` (`KismetMathLibrary.Dot_VectorVector` (0.0 0.0 0.0) (`SceneComponent.GetForwardVector` (`self.Camera`)))) 0.25) (`self.Can Wallrun`))
    (`MovementComponent.SetPlaneConstraintEnabled` _charactermovement true)
    (`MovementComponent.SetPlaneConstraintNormal` _charactermovement (0.0 0.0 0.0))
    (if (`self.Get Wall Direction`)
      (`SceneComponent.K2_SetRelativeRotation` _camera (struct :`Roll` 10.0) false false)
      (else
        (`SceneComponent.K2_SetRelativeRotation` _camera (struct :`Roll` -10.0) false false)))
    (set `CharacterMovementComponent.GravityScale` 0.25 (`self.CharacterMovement`))
    (`self.LaunchCharacter` (`KismetMathLibrary.MakeVector` _returnvalue_x _returnvalue_y (/ (`self._wallrunningInitialForce`) 2.5)) false true)
    (else
      (set `self._wallrunningWall` null)
      (set `self._wallrunningNormal` (0.0 0.0 0.0))
      (return))))

(fn `Toggle Crouch`
  (if (`self._isCrouching`)
    (`CapsuleComponent.SetCapsuleHalfHeight` (`self.CapsuleComponent`) 40.0 true)
    (else
      (`CapsuleComponent.SetCapsuleHalfHeight` (`self.CapsuleComponent`) 88.0 true))))

(fn `Toggle Movement Speed`
  ;[1 1 1] Toggle movement speed - AV
  (if (`self.is_Sprinting`)
    (set `CharacterMovementComponent.MaxWalkSpeed` (`self._walkSpeed`) (`self.CharacterMovement`))
    (else
      (set `CharacterMovementComponent.MaxWalkSpeed` (`self._sprintSpeed`) (`self.CharacterMovement`)))))

(fn `Update Wallrunning`
  (if (`self.Is Wallrunning`)
    (if (not (`self.Can Wallrun`))
      (`self.End Wallrunning` false))))

(fn `UpdateGrapple`
  (bind _returnvalue (`self.K2_GetActorLocation`))
  (bind _returnvalue_2 (`self.GetVelocity`))
  (bind __grappledistance (`self._grappleDistance`))
  (bind _returnvalue_3 (- _returnvalue (`self.K2_GetActorLocation` (`self._grappling`))))
  (bind _returnvalue_4 (`KismetMathLibrary.VSize` _returnvalue_3))
  (bind _returnvalue_5 (`KismetMathLibrary.Normal` _returnvalue_3))
  (`/Engine/EditorBlueprintResources/StandardMacros.IsValid` (`self._grappling`)
    (:`Is Valid`
      (`|ExecutionSequence`
        (:`then_0`
          (`self.K2_SetActorLocation` (`self._grappleCable`) _returnvalue false false)
          (if (> _returnvalue_4 __grappledistance)
            (`self.K2_SetActorLocation` (+ (`self.K2_GetActorLocation`) (* (* (- _returnvalue_4 __grappledistance) _returnvalue_5) (-1.0 -1.0 -1.0))) true)
            (set `MovementComponent.Velocity` (- _returnvalue_2 (* (`KismetMathLibrary.Dot_VectorVector` _returnvalue_2 _returnvalue_5) _returnvalue_5)) (`self.CharacterMovement`))))
        (:`then_1`
          (if (not (`NavMovementComponent.IsFalling` (`self.CharacterMovement`)))
            (`KismetSystemLibrary.PrintString` "c")
            (`self.EndGrapple`)))))))

(fn `UpdateMission`
  (params (newMissionText :type String))
  (`KismetSystemLibrary.PrintString` newMissionText))

(fn `UserConstructionScript`)