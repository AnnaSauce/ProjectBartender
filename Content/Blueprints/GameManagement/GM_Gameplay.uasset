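; GM_Gameplay is a gameplay manager, apparently the game mode, that steps the match through its states and relays points.
; On BeginPlay it caches the game instance and game state, binds to the state dispatcher, and after a delay requests initialisation.
; A state switch advances initialisation to active play after another delay and shows the win screen widget at game end.
; SendPointsToPlayer passes points on through CallReceivePoints.
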(event `self.ReceiveBeginPlay`
  (`KismetSystemLibrary.PrintString` "Gameplay")
  (`self.Init`))

(event `Init`
  ;[1 1 1] InitChain
  (`self.BindGameInstance`)
  (`self.BindGameState`)
  (`KismetSystemLibrary.Delay` 1.0)
  (`/Game/Blueprints/GameManagement/GS_Gamestate.ChangeState` (`self.GS`) "NewEnumerator1"))

(event `BindGameInstance`
  ;[1 1 1] BindGameInstance
  (set `self.GI` (cast `/Game/Blueprints/GameManagement/GI_GameInstance` (`GameplayStatics.GetGameInstance`) :!pure true)))

(event `BindGameState`
  ;[1 1 1] BindGameState
  (bind _output_get (set `self.GS` (cast `/Game/Blueprints/GameManagement/GS_Gamestate` (`GameplayStatics.GetGameState`) :!pure true)))
  (add `/Game/Blueprints/GameManagement/GS_Gamestate.StateDispatcher` _output_get (`|CreateDelegate` :!event `SwitchOnStates`)))

(event `Send Points To Player`
  (params (Points :type Integer))
  ;[1 1 1] PointDispatch
  (`self.Receive Points` Points))

(event `SwitchOnStates`
  (params (newState :type "/Game/Blueprints/GameManagement/E_States Enum" :default "NewEnumerator0"))
  (switch `/Game/Blueprints/GameManagement/E_States` newState
    (:`NewEnumerator1`
      (`KismetSystemLibrary.PrintString` "Init")
      (`KismetSystemLibrary.Delay` 4.0)
      (`/Game/Blueprints/GameManagement/GS_Gamestate.ChangeState` (`self.GS`) "NewEnumerator2"))
    (:`NewEnumerator2`
      (`KismetSystemLibrary.PrintString` "Active"))
    (:`NewEnumerator3`
      (bind _returnvalue (`|CreateWidget` "/Game/UI/WB_WinScreen.WB_WinScreen_C"))
      (`UserWidget.AddToViewport` _returnvalue 0))))

(fn `UserConstructionScript`)