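; GM_GameplayMode is a gameplay game mode that relays points toward the player and hooks into game state changes.
; SendPointsToPlayer prints the awarded amount and passes it on through a ReceivePoints call.
; BindToGameState binds an event to the GS_Gamestate state dispatcher, but BeginPlay is empty and nothing here calls it.
; SwitchOnStates holds a switch on the new state with no branches implemented.
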(event `self.ReceiveBeginPlay`)

(event `BindToGameState`
  ;[1 1 1] BindGameState
  (bind _output_get (set `self.GS` (cast `/Game/Blueprints/GameManagement/GS_Gamestate` (`GameplayStatics.GetGameState`) :!pure true)))
  (add `/Game/Blueprints/GameManagement/GS_Gamestate.StateDispatcher` _output_get (`|CreateDelegate` :!event `SwitchOnStates`)))

(event `Send Points To Player`
  (params (Points :type Integer))
  ;[1 1 1] PointDispatch
  (`KismetSystemLibrary.PrintString` (`KismetStringLibrary.Concat_StrStr` "+" (`KismetStringLibrary.Conv_IntToString` Points) " Points"))
  (`self.Receive Points` Points))

(event `SwitchOnStates`
  (params (newState :type "/Game/Blueprints/GameManagement/E_States Enum" :default "NewEnumerator0"))
  (switch `/Game/Blueprints/GameManagement/E_States` newState))

(fn `UserConstructionScript`)