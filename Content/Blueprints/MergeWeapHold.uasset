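; MergeWeapHold is a weapon holder component that spawns a weapon and relays fire and reload input to it.
; On BeginPlay it spawns WeaponToSpawn using its own relative transform, stores it and attaches it to itself.
; Trigger events start firing with a reticle and direction or cancel it, guarded by a validity check.
; Reload runs only below maximum ammo, without that validity check, and prints a status message either way.
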(event `self.ReceiveBeginPlay`
  (bind _returnvalue (`|SpawnActorFromClass` (`self.WeaponToSpawn`) (`self.GetRelativeTransform`) "AlwaysSpawn" "MultiplyWithRoot" null null))
  (bind _output_get (set `self.Weapon` _returnvalue))
  (`Actor.K2_AttachToComponent` _output_get self "None" "KeepRelative" "KeepRelative" "KeepRelative" true))

(event `TriggerDown`
  (params (Reticle :type "Vector Structure") (Direction :type "Vector Structure"))
  (bind _weapon (`self.Weapon`))
  ;[1 1 1] If there is a weapon, shoot it
  (`/Engine/EditorBlueprintResources/StandardMacros.IsValid` _weapon
    (:`Is Valid`
      (`/Game/Blueprints/Weapons/BP_WeaponBase.Fire` _weapon Reticle Direction))))

(event `TriggerUp`
  (bind _weapon (`self.Weapon`))
  ;[1 1 1] If there is a weapon, shoot it
  (`/Engine/EditorBlueprintResources/StandardMacros.IsValid` _weapon
    (:`Is Valid`
      (`/Game/Blueprints/Weapons/BP_WeaponBase.Cancel Fire` _weapon))))

(event `ReloadPressed`
  (bind _weapon (`self.Weapon`))
  ;[0 0.5176 1] If the weapons current ammo count is less than its max capacity...
  (if (< (`/Game/Blueprints/Weapons/BP_WeaponBase.currentAmmo` _weapon) (`/Game/Blueprints/Weapons/BP_WeaponBase.maxAmmo` _weapon))
    (`/Game/Blueprints/Weapons/BP_WeaponBase.Reload` _weapon)
    (`KismetSystemLibrary.PrintString` "Reloading")
    (else
      (`KismetSystemLibrary.PrintString` "Ammo is already at max capacity"))))