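; Score component that tracks points and an S-to-F grade, with score decay.
; A looping timer drains one point per half second, starting paused and resuming if a single check, three seconds after BeginPlay, finds Score unchanged.
; ChangeScoreBy runs CheckGrade, which switches on Grade to test neighboring thresholds through macros, though each macro assigns SClass.
; The debug print standing in for UI updates is disconnected.
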(event `self.ReceiveBeginPlay`
  (bind _returnvalue (`KismetSystemLibrary.K2_SetTimerDelegate` (delegate `Deteriorate Score`) 0.5 true))
  (bind _output_get (set `self.DeterioratingTimer` _returnvalue))
  (`KismetSystemLibrary.K2_PauseTimerHandle` _output_get)
  (`self.Check For Points`))

(event `Deteriorate Score`
  ;[1 1 1] Decrease Score by 1 every half second
  (if (> (`self.Score`) 0)
    (`self.ChangeScoreBy` -1)))

(event `Check For Points`
  ;[1 1 1] Check if points have been scored in the last 3 seconds
  (set `self.BeforeScore` (`self.Score`))
  (`KismetSystemLibrary.Delay` 3.0)
  (if (== (`self.Score`) (`self.BeforeScore`))
    (`KismetSystemLibrary.K2_UnPauseTimerHandle` (`self.DeterioratingTimer`))))

(fn `ChangeScoreBy`
  (params (Amount :type "Integer (by ref)"))
  (bind _output_get (set `self.Score` (+ (`self.Score`) Amount)))
  (`self.CheckGrade`)
  (return))

(fn `CheckGrade`
  (locals (Thresholds :type "Array of Integer"))
  (switch `/Game/Blueprints/Score/Grade` (`self.Grade`)
    (:`NewEnumerator0`
      (if (< (`self.Score`) 100)
        (set `self.Grade` "NewEnumerator0")))
    (:`NewEnumerator1`
      (if (>= (`self.Score`) 100)
        (set `self.Grade` "NewEnumerator0")
        (elif (< (`self.Score`) 75)
          (set `self.Grade` "NewEnumerator0"))))
    (:`NewEnumerator2`
      (if (>= (`self.Score`) 75)
        (set `self.Grade` "NewEnumerator0")
        (elif (< (`self.Score`) 50)
          (set `self.Grade` "NewEnumerator0"))))
    (:`NewEnumerator3`
      (if (>= (`self.Score`) 50)
        (set `self.Grade` "NewEnumerator0")
        (elif (< (`self.Score`) 25)
          (set `self.Grade` "NewEnumerator0"))))
    (:`NewEnumerator4`
      (if (>= (`self.Score`) 25)
        (set `self.Grade` "NewEnumerator0")))))