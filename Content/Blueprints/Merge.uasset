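; Player pawn Blueprint with Enhanced Input look and movement, a basic health system and a pause menu.
; AnyDamage subtracts from Health and only prints it, with no death handling; the M key applies test damage to itself.
; BeginPlay adds the health widget to the viewport.
; The pause action toggles WB_Pause, switching game pause, input mode and mouse cursor together.
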(event `EnhancedInput|/Game/Input/Action_Look`
  (params (ActionValue :type "Vector2D Structure") (ElapsedSeconds :type "Float (double-precision)") (TriggeredSeconds :type "Float (double-precision)") (InputAction :type "InputAction Object Reference" :default "/Game/Input/Action_Look.Action_Look"))
  ;[1 1 1] Camera control
  (:`Triggered`
    (`self.AddControllerYawInput` ActionValue_X)
    (`self.AddControllerPitchInput` (* ActionValue_Y -1.0))))

(event `EnhancedInput|/Game/Input/Action_Move`
  (params (ActionValue :type "Vector2D Structure") (ElapsedSeconds :type "Float (double-precision)") (TriggeredSeconds :type "Float (double-precision)") (InputAction :type "InputAction Object Reference" :default "/Game/Input/Action_Move.Action_Move"))
  ;[1 1 1] Movement action and Jump action
  (:`Triggered`
    (`self.AddMovementInput` (`self.GetActorRightVector`) ActionValue_X)
    (`self.AddMovementInput` (`self.GetActorForwardVector`) ActionValue_Y)))

(event `self.ReceiveAnyDamage`
  (params (Damage :type "Float (single-precision)") (DamageType :type "DamageType Object Reference") (InstigatedBy :type "Controller Object Reference") (DamageCauser :type "Actor Object Reference"))
  ;[1 1 1] Health System
  (set `self.Health` (- (`self.Health`) Damage))
  (if (<= (`self.Health`) 0.0)
    (`KismetSystemLibrary.PrintString` (`KismetStringLibrary.Conv_DoubleToString` (`self.Health`)))
    (else
      (`KismetSystemLibrary.PrintString` (`KismetStringLibrary.Conv_DoubleToString` (`self.Health`))))))

(event `Key|M`
  (params (Key :type "Key Structure"))
  ;[1 1 1] Experimenting Damage (See if UI works)
  (:`Pressed`
    (`GameplayStatics.ApplyDamage` self 10.0)))

(event `self.ReceiveBeginPlay`
  ;[1 1 1] Health UI
  (bind _returnvalue (`|CreateWidget` "/Game/UI/WB_HealthSystem.WB_HealthSystem_C" (`GameplayStatics.GetPlayerController` 0)))
  (`UserWidget.AddToViewport` _returnvalue 0))

(event `EnhancedInput|/Game/Input/Action_PauseGame`
  (params (ActionValue :type Boolean) (ElapsedSeconds :type "Float (double-precision)") (TriggeredSeconds :type "Float (double-precision)") (InputAction :type "InputAction Object Reference" :default "/Game/Input/Action_PauseGame.Action_PauseGame"))
  (bind _returnvalue (`GameplayStatics.GetPlayerController` 0))
  ;[1 1 1] Pause UI
  (:`Started`
    (if (not (`self.isPauseMenuOpened?`))
      (set `self.isPauseMenuOpened?` true)
      (bind _returnvalue_2 (`|CreateWidget` "/Game/UI/WB_Pause.WB_Pause_C" _returnvalue))
      (bind _output_get (set `self.PauseMenuWB` _returnvalue_2))
      (`UserWidget.AddToViewport` (`self.PauseMenuWB`) 0)
      (`UserWidget.AddToViewport` _output_get 0)
      (`WidgetBlueprintLibrary.SetInputMode_GameAndUIEx` _returnvalue (`self.PauseMenuWB`))
      (set `PlayerController.bShowMouseCursor` true (`GameplayStatics.GetPlayerController` 0))
      (`GameplayStatics.SetGamePaused` true)
      (else
        (set `self.isPauseMenuOpened?` false)
        (`Widget.RemoveFromParent` (`self.PauseMenuWB`))
        (`GameplayStatics.SetGamePaused` false)
        (`WidgetBlueprintLibrary.SetInputMode_GameOnly` _returnvalue)
        (set `PlayerController.bShowMouseCursor` false (`GameplayStatics.GetPlayerController` 0))))))

(fn `UserConstructionScript`)